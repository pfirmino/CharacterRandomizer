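; BP_GameMode is the character randomizer's game mode, bridging a server response to the character customization object.
; RegisterUI stores a CustomizeCharacter reference.
; On HttpResponse, success forwards skin, eye, hair, clothing and body type values to GetRandomFromServer on that reference, while failure calls OnServerFailed.
; The HTTP request itself is not issued in this Blueprint's graphs.
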(event Custom|RegisterUI
  (params (Customize%20Character :type BP%20Customize%20Character%20Object%20Reference))
  (Variables|Default|SetCustomizeCharacter Customize%20Character))

(event EventBeginPlay)

(event EventTick
  (params (DeltaSeconds :type Float%20%28single-precision%29)))

(event EventHttpResponse
  (if (Variables|Default|GetSucceed)
    (Default|GetRandomfromServer (Variables|Default|GetcustomizeCharacter) (Variables|Default|GetSkinColorInt) (Variables|Default|GetEyesColorInt) (Variables|Default|GetHairStyleInt) (Variables|Default|GetHairColorInt) (Variables|Default|GetUpperBodyInt) (Variables|Default|GetLowerBodyInt) (Variables|Default|GetHandsInt) (Variables|Default|GetFeetInt) (Variables|Default|GetBodyTypeFloat))
    (else
      (Default|OnServerFailed (Variables|Default|GetcustomizeCharacter)))))

(fn ConstructionScript)